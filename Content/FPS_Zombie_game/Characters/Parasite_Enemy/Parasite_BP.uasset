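; Parasite enemy character that repeatedly chases the player in a zombie FPS.
; A looping AI MoveTo drives the chase; on reaching the player it triggers a cooldown-gated attack that only prints a debug message, with no damage applied.
; DealDamage reduces health, pausing the chase behind a hit-reaction montage and timed lockout.
; Death ragdolls the mesh, increments the player's frag count and destroys the actor after a delay.
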(event Custom|Chase%20Player
  ;[1 1 1] Enemy AI
  (Development|PrintString "Ai Update")
  (if (or (Variables|Default|GetEnemyDied) (Variables|Default|GetHitAnimPlaying))
    (Development|PrintString "ai stopped")
    (else
      (AI|AIMoveTo self "0, 0, 0" (Game|GetPlayerCharacter 0) 5.0 false
        (:OnSuccess
          (if (Variables|Default|GetCanAttack)
            (Variables|Default|SetCanAttack false)
            (CallFunction|RechargeAttack)
            (CallFunction|ChasePlayer)
            (Utilities|Casting|CastToPlayer_BP (Game|GetPlayerCharacter 0))
            (Development|PrintString "Player Damaged")
            (else
              (CallFunction|ChasePlayer))))
        (:OnFail
          (CallFunction|ChasePlayer))))))

(event Custom|Recharge%20Attack
  ;[1 1 1] Recharge Attack
  (Utilities|FlowControl|Delay (Variables|Default|GetAttackRate))
  (Variables|Default|SetCanAttack true))

(event Custom|DealDamage
  (params (Damage :type Float%20%28single-precision%29))
  ;[1 1 1] Decrement Health
  (bind _output_get (Variables|Default|SetHealth (- (Variables|Default|GetHealth) Damage)))
  (if (<= _output_get 0.0)
    ;[1 1 1] Dead
    (Physics|SetSimulatePhysics (Variables|Character|GetMesh) true)
    (Variables|Default|SetEnemyDied true)
    (bind _asplayer_bp (Utilities|Casting|CastToPlayer_BP (Game|GetPlayerCharacter 0)))
    (Math|Integer|IncrementInt (Variables|/Game/FPS_Zombie_game/Characters/Player/Player_BP.Player_BP_C|GetFragsCount _asplayer_bp)
      (:%20%20
        (Utilities|FlowControl|Delay 3e+01)
        (Actor|DestroyActor)))
    (else
      ;[1 1 1] Hit
      (if (not (Variables|Default|GetHitAnimPlaying))
        (Development|PrintString "trying to stop pawn movement")
        (Components|Movement|StopMovementImmediately (Variables|Character|GetCharacterMovement))
        (Variables|Default|SetHitAnimPlaying true)
        (Development|PrintString "hit anim set true")
        (Animation|Montage|MontagePlay (Components|SkeletalMesh|GetAnimInstance (Variables|Character|GetMesh)) "/Game/FPS_Zombie_game/Characters/Parasite_Enemy/ZombieHitReaction.ZombieHitReaction" 1.0 "MontageLength" 0.0 true)
        (Utilities|FlowControl|Delay 1e+01)
        (Variables|Default|SetHitAnimPlaying false)
        (CallFunction|ChasePlayer)))))

(event EventBeginPlay
  (Variables|Default|SetHealth (Variables|Default|GetMaxHealth))
  (Utilities|FlowControl|Delay 0.2)
  (CallFunction|ChasePlayer))

(fn ConstructionScript)